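; Player character Blueprint that handles camera setup at spawn and opening the pause menu.
; On BeginPlay it blends the first player controller's view to the owner of its Camera and switches to game-only input.
; The Pausa input action creates and shows the Menupausa widget, gives it UI-only input focus with a visible cursor, and pauses the game.
; Resuming is not handled here.
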(event `InputAction|Pausa`
  (params (Key :type "Key Structure"))
  (bind _returnvalue (`GameplayStatics.GetPlayerController` 0))
  ;[1 1 1] PAUSA
  (:`Pressed`
    (bind _returnvalue_2 (`|CreateWidget` "/Game/Unexplored/Blueprints/menupausa.menupausa_C" _returnvalue))
    (`UserWidget.AddToPlayerScreen` _returnvalue_2 0)
    (`WidgetBlueprintLibrary.SetInputMode_UIOnlyEx` _returnvalue _returnvalue_2)
    (set `PlayerController.bShowMouseCursor` true _returnvalue)
    (`GameplayStatics.SetGamePaused` true)))

(event `self.ReceiveBeginPlay`
  (bind _returnvalue (`GameplayStatics.GetPlayerController` 0))
  (`PlayerController.SetViewTargetWithBlend` _returnvalue (`ActorComponent.GetOwner` (`self.Camera`)) 0.1 "VTBlend_Linear" 0.0 false)
  (`WidgetBlueprintLibrary.SetInputMode_GameOnly` _returnvalue))

(fn `UserConstructionScript`)